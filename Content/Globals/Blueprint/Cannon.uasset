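; Cannon actor that fires a projectile when its Fire event is called.
; Fire spawns a muzzle emitter at the Arrow component and triggers the fire animation through the cannon mesh's CannonAnim instance.
; It then spawns a CannonShot at the Arrow's location with an initial velocity along the actor's forward vector, always spawning regardless of collision.
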(event `Fire`
  (`GameplayStatics.SpawnEmitterAtLocation` "/Game/Globals/ParticleSystems/CannonFire.CannonFire" (`SceneComponent.K2_GetComponentLocation` (`self.Arrow`)))
  (`/Game/Globals/Mesh/CannonAnim.PlayFire` (`self.GetCannonAnim`))
  (`|SpawnActorFromClass` "/Game/Globals/Blueprint/CannonShot.CannonShot_C" (`KismetMathLibrary.Conv_VectorToTransform` (`SceneComponent.K2_GetComponentLocation` (`self.Arrow`))) "AlwaysSpawn" "OverrideRootScale" null (* (`KismetMathLibrary.GetForwardVector` (`self.K2_GetActorRotation`)) 1000.0)))

(fn `UserConstructionScript`)