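; A main menu 3D button actor that responds to mouse and touch input on its Box component.
; Cursor and touch events route into shared InputBegan, InputLeft and Clicked events.
; InputBegan enlarges the Box by a configurable amount over the scale saved at BeginPlay, and InputLeft restores it.
; Clicked fires on mouse release or touch end but is an empty hook here.
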(event `self.Box.OnBeginCursorOver`
  (params (TouchedComponent :type "PrimitiveComponent Object Reference"))
  ;[1 1 1] Input Pass Throughs
  (`self.InputBegan`))

(event `self.Box.OnEndCursorOver`
  (params (TouchedComponent :type "PrimitiveComponent Object Reference"))
  ;[1 1 1] Input Pass Throughs
  (`self.InputLeft`))

(event `self.Box.OnReleased`
  (params (TouchedComponent :type "PrimitiveComponent Object Reference") (ButtonReleased :type "Key Structure" :default "AnyKey"))
  ;[1 1 1] Input Pass Throughs
  (`self.Clicked`))

(event `self.Box.OnInputTouchEnter`
  (params (FingerIndex :type "ETouchIndex Enum" :default "Touch1") (TouchedComponent :type "PrimitiveComponent Object Reference"))
  ;[1 1 1] Input Pass Throughs
  (`self.InputBegan` :!label _label))

(event `self.Box.OnInputTouchBegin`
  (params (FingerIndex :type "ETouchIndex Enum" :default "Touch1") (TouchedComponent :type "PrimitiveComponent Object Reference"))
  ;[1 1 1] Input Pass Throughs
  (goto _label))

(event `self.Box.OnInputTouchEnd`
  (params (FingerIndex :type "ETouchIndex Enum" :default "Touch1") (TouchedComponent :type "PrimitiveComponent Object Reference"))
  ;[1 1 1] Input Pass Throughs
  (`self.InputLeft`)
  (`self.Clicked`))

(event `self.Box.OnInputTouchLeave`
  (params (FingerIndex :type "ETouchIndex Enum" :default "Touch1") (TouchedComponent :type "PrimitiveComponent Object Reference"))
  ;[1 1 1] Input Pass Throughs
  (`self.InputLeft`))

(event `self.ReceiveBeginPlay`
  (`PrimitiveComponent.SetCollisionEnabled` (`self.Box`) "QueryAndPhysics")
  (set `self.StartingScale` (`SceneComponent.K2_GetComponentScale` (`self.Box`))))

(event `InputBegan`
  (`SceneComponent.SetWorldScale3D` (`self.Box`) (+ (`self.StartingScale`) (`self.InputOverScaleUp`))))

(event `InputLeft`
  (`SceneComponent.SetWorldScale3D` (`self.Box`) (`self.StartingScale`)))

(event `Clicked`)

(fn `UserConstructionScript`)